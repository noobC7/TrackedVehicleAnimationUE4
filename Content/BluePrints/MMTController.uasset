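; Player controller that handles camera look input, a debug low-FPS mode and on-screen machinery widgets.
; Horizontal and vertical axes feed yaw and pitch input.
; A key toggle caps frame rate through console commands for physics testing and shows an indicator widget, with the cap cleared on BeginPlay.
; Helper functions create machinery widgets into a tracked array and remove all valid ones from their parent.
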(event EventBeginPlay
  ;[1 1 1] Create Low FPS Mode widget
  (bind _returnvalue (UserInterface|CreateWidget "/Game/BluePrints/UMG/LowFPSModeWidget.LowFPSModeWidget_C"))
  (Variables|Default|SetLowFPSModeWidget _returnvalue)
  ;[1 1 1] Low FPS mode for physics testing
  (Development|ExecuteConsoleCommand "t.MaxFPS -1" 0)
  (Variables|Default|SetLowFPSMode false)
  (Widget|RemovefromParent (Variables|Default|GetLowFPSModeWidget)))

(event EventTick
  (params (DeltaSeconds :type Float%20%28single-precision%29)))

(event Input|AxisEvents|InputAxisCameraHorizontal
  (params (AxisValue :type Float%20%28single-precision%29))
  (Class|PlayerController|AddYawInput AxisValue))

(event Input|AxisEvents|InputAxisCameraVertical
  (params (AxisValue :type Float%20%28single-precision%29))
  (Class|PlayerController|AddPitchInput AxisValue))

(event Input|KeyboardEvents|Shift0
  (params (Key :type Key%20Structure :default "None"))
  (bind _lowfpsmodewidget (Variables|Default|GetLowFPSModeWidget))
  ;[1 1 1] Low FPS mode for physics testing
  (:Pressed
    (if (Variables|Default|GetLowFPSMode)
      (Development|ExecuteConsoleCommand "t.MaxFPS -1" 0)
      (Variables|Default|SetLowFPSMode false)
      (Widget|RemovefromParent _lowfpsmodewidget)
      (else
        (Development|ExecuteConsoleCommand "t.MaxFPS 15" 0)
        (Variables|Default|SetLowFPSMode true)
        (UserInterface|Viewport|AddtoViewport _lowfpsmodewidget 0)))))

(fn ConstructionScript)

(fn CreateMachineryWidget
  (params (WidgetClass :type User%20Widget%20Class%20Reference))
  (bind _returnvalue (UserInterface|CreateWidget WidgetClass self))
  (Utilities|Array|Add (Variables|Default|GetMachineryWidget) _returnvalue)
  (UserInterface|Viewport|AddtoViewport _returnvalue 0))

(fn RemoveMachineryWidget
  (for _array_element (Variables|Default|GetMachineryWidget)
    (Utilities|IsValid _array_element
      (:Is%20Valid
        (Widget|RemovefromParent _array_element)))))