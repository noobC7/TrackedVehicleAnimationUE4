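; TCP client Blueprint, named for a MATLAB link in the tracked-vehicle folder, that receives numeric commands from a local socket server.
; On BeginPlay it connects to localhost and tracks the connection ID and state.
; Each message is read as a string into Command, then split and converted by index into the CommandFloat array.
; Status and messages print for debugging; HUDGetCommand is an empty stub.
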(event Custom|connected
  (params (ConnectionId :type Integer))
  (bind _output_get (Variables|Default|SetConnection%20Id ConnectionId))
  (Variables|Default|SetWhetherConnected true)
  (Development|PrintString (Utilities|String|Append "connected with" (Utilities|String|ToString(Integer) _output_get))))

(event Custom|mess
  (params (ConnectionId :type Integer) (Message :type Array%20of%20Bytes))
  ;[1 1 1] 接受命令
  (bind _returnvalue (Class|TcpSocketConnection|MessageReadString Message (Utilities|Array|Length Message)))
  (bind _output_get (Variables|Default|SetCommand _returnvalue))
  (Development|PrintString _output_get)
  (for (_array_element _array_index) (Utilities|String|ParseIntoArray (Variables|Default|GetCommand) " ")
    (Utilities|Array|SetArrayElem (Variables|Default|GetCommand_float) _array_index (Math|Conversions|ToFloat(Integer) _array_element))))

(event Custom|disconnected
  (params (ConnectionId :type Integer))
  (Variables|Default|SetWhetherConnected false)
  (Development|PrintString "disconnected"))

(event EventBeginPlay
  (Class|TcpSocketConnection|Connect "127.0.0.1" 7000 (delegate Custom|disconnected) (delegate Custom|connected) (delegate Custom|mess)))

(fn ConstructionScript)

(fn HUDGetCommand
  (return 0))